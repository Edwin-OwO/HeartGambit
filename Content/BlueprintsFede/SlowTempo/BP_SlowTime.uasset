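; BP_SlowTime toggles a slow-time effect around the player's top-down character through its SlowTimeActive event.
; A FlipFlop alternates between setting global time dilation to Velocity with a compensating player CustomTimeDilation and camera post-processing, and resetting them.
; It also flips CantUseCards, false while active and true after reset.
; Changes run inside loops over BP_SlowTimeExampleCube actors, so they require at least one cube.
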(event `SlowTimeActive`
  (bind _asbp_top_down_character (cast `/Game/TopDown/Blueprints/BP_TopDownCharacter` (`GameplayStatics.GetPlayerPawn` 0)))
  (set `self.Character` _asbp_top_down_character)
  (`/Engine/EditorBlueprintResources/StandardMacros.FlipFlop`
    (:`A`
      (bind _outactors (`GameplayStatics.GetAllActorsOfClass` "/Game/BlueprintsFede/SlowTempo/BP_SlowTimeExampleCube.BP_SlowTimeExampleCube_C"))
      (bind _output_get (set `self.Objects` _outactors))
      (for _array_element _output_get
        (set `self.Actor` _array_element)
        (`GameplayStatics.SetGlobalTimeDilation` (`self.Velocity`))
        (set `Actor.CustomTimeDilation` 10.0 _asbp_top_down_character)
        (set `CameraComponent.PostProcessSettings` (`self.PostProcessing`) (`Actor.GetComponentByClass` (`self.Character`) "/Script/Engine.CameraComponent"))
        (set `self.CantUseCards` false)))
    (:`B`
      (for _array_element_2 (`self.Objects`)
        (set `self.Actor` _array_element_2)
        (`GameplayStatics.SetGlobalTimeDilation` 1.0)
        (set `Actor.CustomTimeDilation` 1.0 _asbp_top_down_character)
        (set `CameraComponent.PostProcessSettings` (struct) (`Actor.GetComponentByClass` (`self.Character`) "/Script/Engine.CameraComponent"))
        (set `self.CantUseCards` true)))))